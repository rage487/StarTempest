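; RapidMoveTo is a behavior tree task that moves a fodder enemy's pawn toward the actor in the TargetToFollow blackboard key.
; On execute, it casts the owner to FodderAIController, caches it for later runs, and calls AIMoveTo with a small acceptance radius.
; It finishes successfully when the move succeeds, with no finish call for a failed move or cast.
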(event `self.ReceiveExecute`
  (params (OwnerActor :type "Actor Object Reference"))
  (if (not (!= (`self.AI_Cont_Ref`) null))
    (bind _asfodder_aicontroller (cast `/Game/BPs/Blueprints/EnemyAI/FodderAIController` OwnerActor))
    (set `self.AI_Cont_Ref` _asfodder_aicontroller))
  (`|AIMoveTo` (`Controller.K2_GetPawn` (`self.AI_Cont_Ref`)) (0.0 0.0 0.0) (`BTFunctionLibrary.GetBlackboardValueAsActor` (`self.TargetToFollow`)) 50.0
    (:`OnSuccess`
      (`self.FinishExecute` true))))
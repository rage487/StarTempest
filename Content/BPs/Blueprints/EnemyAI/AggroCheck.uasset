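; Behavior tree node that gives FodderAI enemies aggro by updating their blackboard target every tick.
; A multi-sphere trace around the pawn gathers nearby objects, ignoring all FodderAI actors, then a Camera-channel line trace tests line of sight to each.
; Visible hits set TargetToFollow and TargetLocation, while blocked ones clear TargetToFollow, so the last result wins.
; An empty sphere trace leaves the blackboard unchanged.
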(event `self.ReceiveTick`
  (params (OwnerActor :type "Actor Object Reference") (DeltaSeconds :type "Float (single-precision)"))
  (bind _returnvalue (`Actor.K2_GetActorLocation` (`Controller.K2_GetPawn` (`self.FodderAIContRef`))))
  (if (not (!= (`self.FodderAIContRef`) null))
    (bind _asfodder_aicontroller (cast `/Game/BPs/Blueprints/EnemyAI/FodderAIController` OwnerActor))
    (set `self.FodderAIContRef` _asfodder_aicontroller))
  (bind _outactors (`GameplayStatics.GetAllActorsOfClass` "/Game/BPs/Blueprints/EnemyAI/FodderAI.FodderAI_C"))
  (set `self.My Location` _returnvalue)
  (bind (_outhits _returnvalue_2) (`KismetSystemLibrary.SphereTraceMultiForObjects` _returnvalue (+ _returnvalue (0.0 0.0 15.0)) 1500.0 (`self.DesiredObjectTypes`) false _outactors))
  (if _returnvalue_2
    (for _array_element _outhits
      (bind (_bblockinghit _binitialoverlap _time _location _impactpoint _normal _impactnormal _physmat _hitactor) (`GameplayStatics.BreakHitResult` _array_element))
      (bind _outhit (`KismetSystemLibrary.LineTraceSingle` (`self.My Location`) (`Actor.K2_GetActorLocation` _hitactor) "TraceTypeQuery2" false _outactors))
      (bind (_bblockinghit_2 _binitialoverlap_2 _time_2 _location_2 _impactpoint_2 _normal_2 _impactnormal_2 _physmat_2 _hitactor_2) (`GameplayStatics.BreakHitResult` _outhit))
      (if (== _hitactor_2 _hitactor) :!label _label
        (`BTFunctionLibrary.SetBlackboardValueAsObject` (`self.TargetToFollow`) _hitactor_2)
        (`BTFunctionLibrary.SetBlackboardValueAsVector` (`self.TargetLocation`) (`Actor.K2_GetActorLocation` _hitactor_2))
        (else
          (`BTFunctionLibrary.SetBlackboardValueAsObject` (`self.TargetToFollow`)))))
    (goto _label)))
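; FodderAI is a simple enemy actor that deals contact damage to the hunter player and can be killed by damage.
; When its cube component begins overlapping a HunterBP, it applies a fixed damage amount to it and destroys itself.
; Incoming damage reduces its AIHealth, and the actor destroys itself once health reaches zero or below.
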(event `self.ReceiveAnyDamage`
  (params (Damage :type "Float (single-precision)") (DamageType :type "DamageType Object Reference") (InstigatedBy :type "Controller Object Reference") (DamageCauser :type "Actor Object Reference"))
  (bind _aihealth (`self.AIHealth`))
  (bind _returnvalue (<= _aihealth 0.0))
  ;[1 1 1] AI Health
  (if _returnvalue
    (`self.K2_DestroyActor` :!label _label)
    (else
      (set `self.AIHealth` (- _aihealth Damage))
      (if _returnvalue
        (goto _label)))))

(event `self.Cube.OnComponentBeginOverlap`
  (params (OverlappedComponent :type "PrimitiveComponent Object Reference") (OtherActor :type "Actor Object Reference") (OtherComp :type "PrimitiveComponent Object Reference") (OtherBodyIndex :type Integer) (bFromSweep :type Boolean) (SweepResult :type "HitResult Structure (by ref)"))
  (bind _ashunter_bp (cast `/Game/BPs/Blueprints/PlayerShipBPs/Hunter/HunterBP` OtherActor))
  (`GameplayStatics.ApplyDamage` _ashunter_bp 50.0)
  (`self.K2_DestroyActor`))

(fn `UserConstructionScript`)
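; Space station actor that offers a ship selection menu on docking and pulls the player character toward itself with a gravity field.
; Overlapping Docking_Radius enables input, letting E open ShipSelectMenu and disable the character's input.
; Leaving Gravity_Field starts the EaseIn timeline, which adjusts character velocity toward the station by offset, curve and GravityStrength.
; The pull stops on leaving GF_Attenuation or entering GravityStop; overlaps are not filtered by actor.
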(event `self.Docking_Radius.OnComponentBeginOverlap`
  (params (OverlappedComponent :type "PrimitiveComponent Object Reference") (OtherActor :type "Actor Object Reference") (OtherComp :type "PrimitiveComponent Object Reference") (OtherBodyIndex :type Integer) (bFromSweep :type Boolean) (SweepResult :type "HitResult Structure (by ref)"))
  ;[1 1 1] ChangeShips
  (`self.EnableInput` (`GameplayStatics.GetPlayerController` 0)))

(event `self.Docking_Radius.OnComponentEndOverlap`
  (params (OverlappedComponent :type "PrimitiveComponent Object Reference") (OtherActor :type "Actor Object Reference") (OtherComp :type "PrimitiveComponent Object Reference") (OtherBodyIndex :type Integer))
  ;[1 1 1] ChangeShips
  (`self.DisableInput` (`GameplayStatics.GetPlayerController` 0)))

(event `Key|E`
  (params (Key :type "Key Structure"))
  ;[1 1 1] ChangeShips
  (:`Pressed`
    (bind _returnvalue (`|CreateWidget` "/Game/Menus/ShipSelectMenu/ShipSelectMenu.ShipSelectMenu_C"))
    (`UserWidget.AddToViewport` _returnvalue 0)
    (`self.DisableInput` (`GameplayStatics.GetPlayerCharacter` 0) (`GameplayStatics.GetPlayerController` 0))))

(event `self.ReceiveTick`
  (params (DeltaSeconds :type "Float (single-precision)"))
  ;[1 1 1] ChangeShips
)

(event `self.Gravity_Field.OnComponentEndOverlap`
  (params (OverlappedComponent :type "PrimitiveComponent Object Reference") (OtherActor :type "Actor Object Reference") (OtherComp :type "PrimitiveComponent Object Reference") (OtherBodyIndex :type Integer))
  (bind _returnvalue (`GameplayStatics.GetPlayerCharacter` 0))
  ;[1 1 1] Make Gravity Fields Work
  (bind (_direction _easein) (`Timeline|EaseIn` :!via `PlayFromStart` :!label _label)
    (:`Update`
      (bind _returnvalue_2 (* _easein (`self.GravityStrength`)))
      (set `MovementComponent.Velocity` (- (`self.GetVelocity` _returnvalue) (* (- (`self.K2_GetActorLocation` _returnvalue) (`self.K2_GetActorLocation`)) (`KismetMathLibrary.MakeVector` _returnvalue_2 _returnvalue_2 _returnvalue_2))) (`Pawn.GetMovementComponent` _returnvalue)))))

(event `self.GF_Attenuation.OnComponentEndOverlap`
  (params (OverlappedComponent :type "PrimitiveComponent Object Reference") (OtherActor :type "Actor Object Reference") (OtherComp :type "PrimitiveComponent Object Reference") (OtherBodyIndex :type Integer))
  ;[1 1 1] Make Gravity Fields Work
  (goto _label :!via `Stop`))

(event `self.Gravity Stop.OnComponentBeginOverlap`
  (params (OverlappedComponent :type "PrimitiveComponent Object Reference") (OtherActor :type "Actor Object Reference") (OtherComp :type "PrimitiveComponent Object Reference") (OtherBodyIndex :type Integer) (bFromSweep :type Boolean) (SweepResult :type "HitResult Structure (by ref)"))
  ;[1 1 1] Make Gravity Fields Work
  (goto _label :!via `Stop`))

(fn `UserConstructionScript`)
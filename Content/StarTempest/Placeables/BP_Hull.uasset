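; BP_Hull is a placeable pickup that restores hull to the player's ship in StarTempest.
; When an actor overlaps PickupRadius, it switches on the CurrentShip of the PC_TopDown controller and continues only if that actor casts to the matching ship Blueprint.
; All ten ship cases share one path that spawns particle and sound effects, adds HullValue to the controller's CurrentHull clamped to MaxHull, then destroys the pickup.
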(event `self.PickupRadius.OnComponentBeginOverlap`
  (params (OverlappedComponent :type "PrimitiveComponent Object Reference") (OtherActor :type "Actor Object Reference") (OtherComp :type "PrimitiveComponent Object Reference") (OtherBodyIndex :type Integer) (bFromSweep :type Boolean) (SweepResult :type "HitResult Structure (by ref)"))
  ;[1 1 1] Player Collecting the Hull
  (bind _aspc_top_down (cast `/Game/StarTempest/Core/PC_TopDown` (`GameplayStatics.GetPlayerController` 0)))
  (switch `/Game/StarTempest/Characters/PlayerShips/E_PlayerShips` (`/Game/StarTempest/Core/PC_TopDown.CurrentShip` _aspc_top_down)
    (:`NewEnumerator0`
      (cast `/Game/StarTempest/Characters/PlayerShips/Corsair/BP_Corsair` OtherActor))
    (:`NewEnumerator1`
      (cast `/Game/StarTempest/Characters/PlayerShips/Crusader/BP_Crusader` OtherActor))
    (:`NewEnumerator2`
      (cast `/Game/StarTempest/Characters/PlayerShips/Dragonfly/BP_Dragonfly` OtherActor))
    (:`NewEnumerator9`
      (cast `/Game/StarTempest/Characters/PlayerShips/Excelsior/BP_Excelsior` OtherActor))
    (:`NewEnumerator3`
      (cast `/Game/StarTempest/Characters/PlayerShips/Hunter/BP_Hunter` OtherActor))
    (:`NewEnumerator4`
      (cast `/Game/StarTempest/Characters/PlayerShips/Juggernaut/BP_Juggernaut` OtherActor))
    (:`NewEnumerator5`
      (cast `/Game/StarTempest/Characters/PlayerShips/Nebula/BP_Nebula` OtherActor))
    (:`NewEnumerator6`
      (cast `/Game/StarTempest/Characters/PlayerShips/Reaper/BP_Reaper` OtherActor))
    (:`NewEnumerator7`
      (cast `/Game/StarTempest/Characters/PlayerShips/Spectre/BP_Spectre` OtherActor))
    (:`NewEnumerator8`
      (cast `/Game/StarTempest/Characters/PlayerShips/Voidwalker/BP_Voidwalker` OtherActor)))
  (`GameplayStatics.SpawnEmitterAtLocation` (`self.HullPickupParticle`) (`self.K2_GetActorLocation`))
  (`GameplayStatics.SpawnSoundAtLocation` (`self.HullPickupSound`) (`self.K2_GetActorLocation`))
  (set `/Game/StarTempest/Core/PC_TopDown.CurrentHull` (`KismetMathLibrary.FClamp` (+ (`/Game/StarTempest/Core/PC_TopDown.CurrentHull` _aspc_top_down) (`self.HullValue`)) 0.0 (`/Game/StarTempest/Core/PC_TopDown.MaxHull` _aspc_top_down)) _aspc_top_down)
  (`self.K2_DestroyActor`))

(fn `UserConstructionScript`)
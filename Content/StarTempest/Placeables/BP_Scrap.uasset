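; BP_Scrap is a placeable scrap pickup that adds to the player's scrap total when the player ship touches it.
; An overlap on PickupRadius requires the controller to be PC_TopDown and the other actor to be BP_PlayerShip.
; It then spawns a pickup particle and sound at its location, adds ScrapValue to the controller's ScrapTotal and destroys itself.
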(event `self.PickupRadius.OnComponentBeginOverlap`
  (params (OverlappedComponent :type "PrimitiveComponent Object Reference") (OtherActor :type "Actor Object Reference") (OtherComp :type "PrimitiveComponent Object Reference") (OtherBodyIndex :type Integer) (bFromSweep :type Boolean) (SweepResult :type "HitResult Structure (by ref)"))
  ;[1 1 1] Player Collecting the Scrap
  (bind _aspc_top_down (cast `/Game/StarTempest/Core/PC_TopDown` (`GameplayStatics.GetPlayerController` 0)))
  (cast `/Game/StarTempest/Characters/PlayerShip/BP_PlayerShip` OtherActor)
  (`GameplayStatics.SpawnEmitterAtLocation` (`self.ScrapPickupParticle`) (`self.K2_GetActorLocation`))
  (`GameplayStatics.SpawnSoundAtLocation` (`self.ScrapPickupSound`) (`self.K2_GetActorLocation`))
  (set `/Game/StarTempest/Core/PC_TopDown.ScrapTotal` (+ (`/Game/StarTempest/Core/PC_TopDown.ScrapTotal` _aspc_top_down) (`self.ScrapValue`)) _aspc_top_down)
  (`self.K2_DestroyActor`))

(fn `UserConstructionScript`)
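; BP_HoverComponent is a component that makes its owning actor's physics body hover above surfaces.
; BeginPlay caches the owner's first PrimitiveComponent.
; A custom event traces down on the Visibility channel and, on a hit, pushes along the surface normal with force fading linearly to zero at trace length.
; The same hit applies linear and angular damping, which is never reset on a miss.
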(event `self.ReceiveBeginPlay`
  (set `self.PrimitiveComponentRef` (`|GetArrayItem` (`Actor.K2_GetComponentsByClass` (`self.GetOwner`) "/Script/Engine.PrimitiveComponent"))))

(event `CustomEvent`
  (params (DeltaSeconds :type "Float (double-precision)"))
  (bind _returnvalue (`SceneComponent.K2_GetComponentLocation` (`self.PrimitiveComponentRef`)))
  (bind (_outhit _returnvalue_2) (`KismetSystemLibrary.LineTraceSingle` _returnvalue (- _returnvalue (`KismetMathLibrary.MakeVector` 0.0 0.0 (`self.Trace Length`))) "TraceTypeQuery1"))
  (if _returnvalue_2
    (bind (_bblockinghit _binitialoverlap _time _location _impactpoint _normal _impactnormal) (`GameplayStatics.BreakHitResult` _outhit))
    (`PrimitiveComponent.AddForce` (`self.PrimitiveComponentRef`) (* _impactnormal (`KismetMathLibrary.Lerp` (`self.HoverForce`) 0.0 (/ (`KismetMathLibrary.VSize` (- _location (`SceneComponent.K2_GetComponentLocation` (`self.PrimitiveComponentRef`)))) (`self.Trace Length`)))) "None" false)
    (`PrimitiveComponent.SetLinearDamping` (`self.PrimitiveComponentRef`) (`self.LinearDamping`))
    (`PrimitiveComponent.SetAngularDamping` (`self.PrimitiveComponentRef`) (`self.AngularDamping`))))
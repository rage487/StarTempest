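; BP_Armor is a placeable armor pickup that the player's ship collects in StarTempest.
; When a BP_PlayerShip overlaps its PickupRadius, it spawns a particle and sound at its location, then destroys itself after granting armor.
; It adds ArmorValue to CurrentArmor on the PC_TopDown player controller, clamped between zero and a quarter of that controller's MaxHull.
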(event `self.PickupRadius.OnComponentBeginOverlap`
  (params (OverlappedComponent :type "PrimitiveComponent Object Reference") (OtherActor :type "Actor Object Reference") (OtherComp :type "PrimitiveComponent Object Reference") (OtherBodyIndex :type Integer) (bFromSweep :type Boolean) (SweepResult :type "HitResult Structure (by ref)"))
  ;[1 1 1] Player Collecting the Armor
  (bind _aspc_top_down (cast `/Game/StarTempest/Core/PC_TopDown` (`GameplayStatics.GetPlayerController` 0)))
  (cast `/Game/StarTempest/Characters/PlayerShip/BP_PlayerShip` OtherActor)
  (`GameplayStatics.SpawnEmitterAtLocation` (`self.ArmorPickupParticle`) (`self.K2_GetActorLocation`))
  (`GameplayStatics.SpawnSoundAtLocation` (`self.ArmorPickupSound`) (`self.K2_GetActorLocation`))
  (set `/Game/StarTempest/Core/PC_TopDown.CurrentArmor` (`KismetMathLibrary.FClamp` (+ (`/Game/StarTempest/Core/PC_TopDown.CurrentArmor` _aspc_top_down) (`self.ArmorValue`)) 0.0 (* (`/Game/StarTempest/Core/PC_TopDown.MaxHull` _aspc_top_down) 0.25)) _aspc_top_down)
  (`self.K2_DestroyActor`))

(fn `UserConstructionScript`)
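; Spitter enemy AI that wanders around the space station's gravity field at fixed height while rotating to face the player every tick.
; An overlap on its detector moves it to a random point near the player before it resumes wandering.
; If the overlapping actor is the player ship, it also fires one delayed fodder shot and a later spitter shot.
; Damage drains health until GM_TopDown handles its death; ramming logic is disconnected.
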(event `self.ReceiveTick`
  (params (DeltaSeconds :type "Float (single-precision)"))
  (`self.K2_SetActorRotation` (`KismetMathLibrary.FindLookAtRotation` (`self.K2_GetActorLocation`) (`self.K2_GetActorLocation` (`GameplayStatics.GetPlayerCharacter` 0)))))

(event `self.ReceiveBeginPlay`
  ;[1 1 1] AI Movement
  (`self.MoveToRandomLocation`))

(event `MoveToRandomLocation`
  (bind _spacestation (`self.SpaceStation`))
  (bind _randomlocation (`NavigationSystem.K2_GetRandomLocationInNavigableRadius` (`self.K2_GetActorLocation` _spacestation) (`SphereComponent.GetScaledSphereRadius` (`/Game/StarTempest/Characters/SpaceStation/BP_SpaceStation.Gravity_Field` _spacestation))))
  ;[1 1 1] AI Movement
  (`|AIMoveTo` self (`KismetMathLibrary.MakeVector` (.x _randomlocation) (.y _randomlocation) 200.0) null 5.0 true
    (:`OnSuccess`
      (`self.MoveToRandomLocation`))))

(event `self.PlayerDetector.OnComponentBeginOverlap`
  (params (OverlappedComponent :type "PrimitiveComponent Object Reference") (OtherActor :type "Actor Object Reference") (OtherComp :type "PrimitiveComponent Object Reference") (OtherBodyIndex :type Integer) (bFromSweep :type Boolean) (SweepResult :type "HitResult Structure (by ref)"))
  (bind _returnvalue (`self.K2_GetActorLocation`))
  (bind _returnvalue_2 (`self.K2_GetActorLocation`))
  (bind _randomlocation (`NavigationSystem.K2_GetRandomLocationInNavigableRadius` (`self.K2_GetActorLocation` (`Controller.K2_GetPawn` (`GameplayStatics.GetPlayerController` 0))) 1000.0))
  ;[1 1 1] Basic Shooting at Player
  (`|ExecutionSequence`
    (:`then_0`
      (cast `/Game/StarTempest/Characters/PlayerShip/BP_PlayerShip` OtherActor)
      (`KismetSystemLibrary.Delay` 0.75)
      (`|SpawnActorFromClass` "/Game/StarTempest/Characters/FodderParent/BP_FodderWep.BP_FodderWep_C" (`KismetMathLibrary.MakeTransform` (+ _returnvalue (0.0 0.0 0.0)) (`KismetMathLibrary.FindLookAtRotation` _returnvalue (`self.K2_GetActorLocation` (`GameplayStatics.GetPlayerCharacter` 0)))) "Undefined" "OverrideRootScale" null null))
    (:`then_1`
      ;[1 1 1] Shoot Spitter Shot
      (cast `/Game/StarTempest/Characters/PlayerShip/BP_PlayerShip` OtherActor)
      (`KismetSystemLibrary.Delay` 2.0)
      (`|SpawnActorFromClass` "/Game/StarTempest/Characters/Enemies/Kinetic/Spitter/BP_SpitterWep.BP_SpitterWep_C" (`KismetMathLibrary.MakeTransform` (+ _returnvalue_2 (0.0 0.0 0.0)) (`KismetMathLibrary.FindLookAtRotation` _returnvalue_2 (`self.K2_GetActorLocation` (`GameplayStatics.GetPlayerCharacter` 0)))) "Undefined" "OverrideRootScale" null null))
    (:`then_2`
      ;[1 1 1] Move Around Player
      (`|AIMoveTo` self (`KismetMathLibrary.MakeVector` (.x _randomlocation) (.y _randomlocation) 200.0) null 5.0 true
        (:`OnSuccess`
          (`self.MoveToRandomLocation`))))))

(event `self.ReceiveAnyDamage`
  (params (Damage :type "Float (single-precision)") (DamageType :type "DamageType Object Reference") (InstigatedBy :type "Controller Object Reference") (DamageCauser :type "Actor Object Reference"))
  ;[1 1 1] Spitter Taking Damage
  (set `self.AIHealth` (- (`self.AIHealth`) Damage))
  (if (<= (`self.AIHealth`) 0.0)
    (`self.CallDeathFunction`)))

(event `self.Cube.OnComponentBeginOverlap`
  (params (OverlappedComponent :type "PrimitiveComponent Object Reference") (OtherActor :type "Actor Object Reference") (OtherComp :type "PrimitiveComponent Object Reference") (OtherBodyIndex :type Integer) (bFromSweep :type Boolean) (SweepResult :type "HitResult Structure (by ref)"))
  ;[1 0 0.02246] Spitter Collision with Player (Off)
)

(fn `CallDeathFunction`
  (bind _asgm_top_down (cast `/Game/StarTempest/Core/GM_TopDown` (`GameplayStatics.GetGameMode`)))
  (`/Game/StarTempest/Core/GM_TopDown.EnemyDestroyedEvent` _asgm_top_down (`self.DeathParticle`) (`self.DeathSound`) (`self.EnemyType`) (`self.GetTransform`) self))

(fn `UserConstructionScript`)

(fn `WepLoop`)
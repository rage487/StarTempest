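; Fodder enemy AI that roams near the space station, faces the player and shoots at them.
; It chains AI moves to random navigable points within the station's gravity field radius, repeating on success.
; A player ship entering its detector triggers one delayed BP_FodderWep shot.
; The game mode calculates incoming damage and handles death through EnemyDestroyedEvent; ramming damage is disconnected.
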(event `self.ReceiveBeginPlay`
  (bind _asgm_top_down (cast `/Game/StarTempest/Core/GM_TopDown` (`GameplayStatics.GetGameMode`)))
  (set `self.GMRef` _asgm_top_down)
  ;[1 1 1] AI Movement
  (`self.MoveToRandomLocation`))

(event `self.ReceiveTick`
  (params (DeltaSeconds :type "Float (single-precision)"))
  (bind _returnvalue (`Controller.K2_GetPawn` (`GameplayStatics.GetPlayerController` 0)))
  (bind (_returnvalue_roll _returnvalue_pitch _returnvalue_yaw) (`KismetMathLibrary.BreakRotator` (`KismetMathLibrary.FindLookAtRotation` (`self.K2_GetActorLocation`) (`self.K2_GetActorLocation` _returnvalue))))
  (if (`KismetSystemLibrary.IsValid` _returnvalue)
    (`self.K2_SetActorRotation` (`KismetMathLibrary.MakeRotator` _returnvalue_roll _returnvalue_pitch (- _returnvalue_yaw 90.0)))))

(event `MoveToRandomLocation`
  (bind _spacestation (`self.SpaceStation`))
  (bind _randomlocation (`NavigationSystem.K2_GetRandomLocationInNavigableRadius` (`self.K2_GetActorLocation` _spacestation) (`SphereComponent.GetScaledSphereRadius` (`/Game/StarTempest/Characters/SpaceStation/BP_SpaceStation.Gravity_Field` _spacestation))))
  ;[1 1 1] AI Movement
  (`|AIMoveTo` self (`KismetMathLibrary.MakeVector` (.x _randomlocation) (.y _randomlocation) 200.0)
    (:`OnSuccess`
      (`self.MoveToRandomLocation`))))

(event `self.PlayerDetector.OnComponentBeginOverlap`
  (params (OverlappedComponent :type "PrimitiveComponent Object Reference") (OtherActor :type "Actor Object Reference") (OtherComp :type "PrimitiveComponent Object Reference") (OtherBodyIndex :type Integer) (bFromSweep :type Boolean) (SweepResult :type "HitResult Structure (by ref)"))
  (bind _returnvalue (`self.K2_GetActorLocation`))
  ;[1 1 1] Detecting and shooting at player
  (cast `/Game/StarTempest/Characters/PlayerShip/BP_PlayerShip` OtherActor)
  (`KismetSystemLibrary.Delay` 1.0)
  (if (`KismetSystemLibrary.IsValid` (`GameplayStatics.GetPlayerPawn` 0))
    (`|SpawnActorFromClass` "/Game/StarTempest/Characters/Enemies/FodderParent/BP_FodderWep.BP_FodderWep_C" (`KismetMathLibrary.MakeTransform` (+ _returnvalue (0.0 0.0 0.0)) (`KismetMathLibrary.FindLookAtRotation` _returnvalue (`self.K2_GetActorLocation` (`GameplayStatics.GetPlayerCharacter` 0)))) "Undefined" "OverrideRootScale" null null)))

(event `self.ReceiveAnyDamage`
  (params (Damage :type "Float (single-precision)") (DamageType :type "DamageType Object Reference") (InstigatedBy :type "Controller Object Reference") (DamageCauser :type "Actor Object Reference"))
  ;[1 1 1] Fodder Taking Damage
  (bind _outgoingdamageamount (`/Game/StarTempest/Core/GM_TopDown.TakingDamage` (`self.GMRef`) (`self.DamageType`) DamageType Damage))
  (set `self.AIHealth` (- (`self.AIHealth`) _outgoingdamageamount))
  (if (<= (`self.AIHealth`) 0.0)
    (`self.CallDeathFunction`)))

(event `self.Cube.OnComponentBeginOverlap`
  (params (OverlappedComponent :type "PrimitiveComponent Object Reference") (OtherActor :type "Actor Object Reference") (OtherComp :type "PrimitiveComponent Object Reference") (OtherBodyIndex :type Integer) (bFromSweep :type Boolean) (SweepResult :type "HitResult Structure (by ref)"))
  ;[1 0 0.02246] Fodder Collision with Player (Off)
)

(fn `CallDeathFunction`
  (bind _asgm_top_down (cast `/Game/StarTempest/Core/GM_TopDown` (`GameplayStatics.GetGameMode`)))
  (`/Game/StarTempest/Core/GM_TopDown.EnemyDestroyedEvent` _asgm_top_down (`self.DeathParticle`) (`self.DeathSound`) (`self.EnemyTier`) (`self.GetTransform`) self))

(fn `UserConstructionScript`)

(fn `WepLoop`)
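; BP_FodderSpawner is an enemy spawner that periodically creates CBP_EFodder enemies around itself.
; From BeginPlay, while CanSpawn is true, it spawns one at a random navigable point within the SpawningRadius sphere, then re-triggers itself after a fixed delay.
; Each spawn receives the BP_SpaceStation actors found in the level.
; The construction script sizes the sphere from the SpawnRadius variable.
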(event `ContinueSpawningEvent`
  (if (`self.CanSpawn`) :!label _label
    (bind _outactors (`GameplayStatics.GetAllActorsOfClass` "/Game/StarTempest/Characters/SpaceStation/BP_SpaceStation.BP_SpaceStation_C"))
    (`|SpawnActorFromClass` "/Game/StarTempest/Characters/Enemies/Energy/EnergyFodder/CBP_EFodder.CBP_EFodder_C" (`KismetMathLibrary.MakeTransform` (`NavigationSystem.K2_GetRandomLocationInNavigableRadius` (`self.K2_GetActorLocation`) (`SphereComponent.SphereRadius` (`self.SpawningRadius`)))) "Undefined" "OverrideRootScale" null _outactors null)
    (`KismetSystemLibrary.Delay` 10.0)
    (`self.ContinueSpawningEvent`)))

(event `self.ReceiveBeginPlay`
  (goto _label))

(fn `UserConstructionScript`
  (`SphereComponent.SetSphereRadius` (`self.SpawningRadius`) (`self.SpawnRadius`) true))
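; BP_DeathsHead is a fodder enemy in StarTempest that dies when its health runs out or it rams the player.
; Incoming damage reduces AIHealth, while overlapping BP_PlayerShip deals heavy damage to the ship and zeroes the enemy's health.
; Both paths call CallDeathFunction, which hands its particle, sound, type, transform and self-reference to GM_TopDown's EnemyDestroyedEvent, delegating death handling to the game mode.
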(event `self.ReceiveAnyDamage`
  (params (Damage :type "Float (single-precision)") (DamageType :type "DamageType Object Reference") (InstigatedBy :type "Controller Object Reference") (DamageCauser :type "Actor Object Reference"))
  ;[1 1 1] Fodder Taking Damage
  (set `self.AIHealth` (- (`self.AIHealth`) Damage))
  (if (<= (`self.AIHealth`) 0.0)
    (`self.CallDeathFunction`)))

(event `self.Cube.OnComponentBeginOverlap`
  (params (OverlappedComponent :type "PrimitiveComponent Object Reference") (OtherActor :type "Actor Object Reference") (OtherComp :type "PrimitiveComponent Object Reference") (OtherBodyIndex :type Integer) (bFromSweep :type Boolean) (SweepResult :type "HitResult Structure (by ref)"))
  ;[1 1 1] Fodder Collision with Player
  (cast `/Game/StarTempest/Characters/PlayerShip/BP_PlayerShip` OtherActor)
  (`GameplayStatics.ApplyDamage` OtherActor 1000.0 (`GameplayStatics.GetPlayerController` 0) self)
  (set `self.AIHealth` 0.0)
  (if (<= (`self.AIHealth`) 0.0)
    (`self.CallDeathFunction`)))

(fn `CallDeathFunction`
  (bind _asgm_top_down (cast `/Game/StarTempest/Core/GM_TopDown` (`GameplayStatics.GetGameMode`)))
  (`/Game/StarTempest/Core/GM_TopDown.EnemyDestroyedEvent` _asgm_top_down (`self.DeathParticle`) (`self.DeathSound`) (`self.EnemyType`) (`self.GetTransform`) self))

(fn `UserConstructionScript`)
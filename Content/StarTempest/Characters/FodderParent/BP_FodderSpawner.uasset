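; Spawner actor that populates navigable area around itself with BP_FodderAI enemies, up to a spawn limit.
; From BeginPlay, a self-recursing, delayed event spawns each fodder at random navmesh XY and fixed height, passes it the space station reference and starts it wandering.
; It prunes invalid entries after each delay; the loop ends once spawning is disabled or the limit is reached.
; The construction script sizes the spawn sphere from SpawnRadius.
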(event `ContinueSpawningEvent`
  (bind _spawnedfodders (`self.SpawnedFodders`))
  (bind _randomlocation (`NavigationSystem.K2_GetRandomLocationInNavigableRadius` (`self.K2_GetActorLocation`) (`SphereComponent.SphereRadius` (`self.SpawningRadius`))))
  (if (`self.CanSpawn`) :!label _label
    (if (not (>= (`KismetArrayLibrary.Array_Length` (`self.SpawnedFodders`)) (`self.Spawn Limit`)))
      (bind _returnvalue (`|SpawnActorFromClass` "/Game/StarTempest/Characters/FodderParent/BP_FodderAI.BP_FodderAI_C" (`KismetMathLibrary.MakeTransform` (`KismetMathLibrary.MakeVector` (.x _randomlocation) (.y _randomlocation) 200.0)) "AdjustIfPossibleButAlwaysSpawn" "OverrideRootScale" null (`self.SpaceStationRef`) null))
      (`KismetArrayLibrary.Array_Add` (`self.SpawnedFodders`) _returnvalue)
      (set `/Game/StarTempest/Characters/FodderParent/BP_FodderAI.SpaceStation` (`self.SpaceStationRef`) _returnvalue)
      (`/Game/StarTempest/Characters/FodderParent/BP_FodderAI.MoveToRandomLocation` _returnvalue)
      (`KismetSystemLibrary.Delay` (`self.Spawn Delay`))
      (for (_array_element _array_index) _spawnedfodders
        (if (not (`KismetSystemLibrary.IsValid` _array_element))
          (`KismetArrayLibrary.Array_Remove` _spawnedfodders _array_index)))
      (`self.ContinueSpawningEvent`))))

(event `self.ReceiveBeginPlay`
  (goto _label))

(fn `UserConstructionScript`
  (`SphereComponent.SetSphereRadius` (`self.SpawningRadius`) (`self.SpawnRadius`) true))
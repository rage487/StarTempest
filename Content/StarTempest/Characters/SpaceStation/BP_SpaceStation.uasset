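; Space station Blueprint that acts as a checkpoint, ship-change dock and gravity well for the player.
; Entering the docking radius saves the player's transform to GM_TopDown and enables input, letting E open a reusable ship select menu and disable character input.
; Leaving the gravity field starts an ease-in timeline that pulls player velocity toward the station, scaled by offset and GravityStrength.
; Exiting the attenuation volume or entering GravityStop halts the pull.
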(event `self.Docking_Radius.OnComponentBeginOverlap`
  (params (OverlappedComponent :type "PrimitiveComponent Object Reference") (OtherActor :type "Actor Object Reference") (OtherComp :type "PrimitiveComponent Object Reference") (OtherBodyIndex :type Integer) (bFromSweep :type Boolean) (SweepResult :type "HitResult Structure (by ref)"))
  ;[1 1 1] Open PlayerShipChange Menu and Set PlayerCheckpoint
  (`self.EnableInput` (`GameplayStatics.GetPlayerController` 0))
  (bind _asgm_top_down (cast `/Game/StarTempest/Core/GM_TopDown` (`GameplayStatics.GetGameMode`)))
  (set `/Game/StarTempest/Core/GM_TopDown.PlayerCheckpointTransform` (`SceneComponent.K2_GetComponentToWorld` (`Character.CapsuleComponent` (`GameplayStatics.GetPlayerCharacter` 0))) _asgm_top_down))

(event `self.Docking_Radius.OnComponentEndOverlap`
  (params (OverlappedComponent :type "PrimitiveComponent Object Reference") (OtherActor :type "Actor Object Reference") (OtherComp :type "PrimitiveComponent Object Reference") (OtherBodyIndex :type Integer))
  ;[1 1 1] Open PlayerShipChange Menu and Set PlayerCheckpoint
  (`self.DisableInput` (`GameplayStatics.GetPlayerController` 0)))

(event `Key|E`
  (params (Key :type "Key Structure"))
  (bind _shipselectmenuref (`self.ShipSelectMenuRef`))
  ;[1 1 1] Open PlayerShipChange Menu and Set PlayerCheckpoint
  (:`Released`
    (if (`KismetSystemLibrary.IsValid` _shipselectmenuref)
      (if (not (`Widget.IsInViewport` _shipselectmenuref))
        (`UserWidget.AddToViewport` (`self.ShipSelectMenuRef`) 0)
        (`self.DisableInput` (`GameplayStatics.GetPlayerCharacter` 0) (`GameplayStatics.GetPlayerController` 0) :!label _label))
      (else
        (bind _returnvalue (`|CreateWidget` "/Game/StarTempest/Core/WBP_ShipSelectMenu.WBP_ShipSelectMenu_C"))
        (bind _output_get (set `self.ShipSelectMenuRef` _returnvalue))
        (`UserWidget.AddToViewport` _output_get 0)
        (goto _label)))))

(event `self.Gravity_Field.OnComponentEndOverlap`
  (params (OverlappedComponent :type "PrimitiveComponent Object Reference") (OtherActor :type "Actor Object Reference") (OtherComp :type "PrimitiveComponent Object Reference") (OtherBodyIndex :type Integer))
  (bind _returnvalue (`GameplayStatics.GetPlayerCharacter` 0))
  ;[1 1 1] Make Gravity Fields Work
  (if (`KismetSystemLibrary.IsValid` (`GameplayStatics.GetPlayerCharacter` 0))
    (bind (_direction _easein) (`Timeline|EaseIn` :!via `PlayFromStart` :!label _label_2)
      (:`Update`
        (bind _returnvalue_2 (* _easein (`self.GravityStrength`)))
        (set `MovementComponent.Velocity` (- (`self.GetVelocity` _returnvalue) (* (- (`self.K2_GetActorLocation` _returnvalue) (`self.K2_GetActorLocation`)) (`KismetMathLibrary.MakeVector` _returnvalue_2 _returnvalue_2 _returnvalue_2))) (`Pawn.GetMovementComponent` _returnvalue))))))

(event `self.GF_Attenuation.OnComponentEndOverlap`
  (params (OverlappedComponent :type "PrimitiveComponent Object Reference") (OtherActor :type "Actor Object Reference") (OtherComp :type "PrimitiveComponent Object Reference") (OtherBodyIndex :type Integer))
  ;[1 1 1] Make Gravity Fields Work
  (goto _label_2 :!via `Stop`))

(event `self.Gravity Stop.OnComponentBeginOverlap`
  (params (OverlappedComponent :type "PrimitiveComponent Object Reference") (OtherActor :type "Actor Object Reference") (OtherComp :type "PrimitiveComponent Object Reference") (OtherBodyIndex :type Integer) (bFromSweep :type Boolean) (SweepResult :type "HitResult Structure (by ref)"))
  ;[1 1 1] Make Gravity Fields Work
  (goto _label_2 :!via `Stop`))

(event `self.ReceiveBeginPlay`
  ;[1 1 1] Make Gravity Fields Work
  (goto _label_2 :!via `Stop`))

(fn `UserConstructionScript`)
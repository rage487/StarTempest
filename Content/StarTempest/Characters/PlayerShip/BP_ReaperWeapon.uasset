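; Short-lived beam weapon actor that fires from the player ship toward the mouse cursor and damages what it hits.
; BeginPlay caches the ship mesh location, then joins the Tick chain that line-traces to the point under the cursor.
; Each pass applies weapon damage on a hit and updates the ReaperBeam particle endpoints.
; The actor destroys itself after a brief delay, so damage can repeat every frame until then.
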(event `self.ReceiveTick`
  (params (DeltaSeconds :type "Float (single-precision)"))
  (bind (_bblockinghit _binitialoverlap _time _location) (`GameplayStatics.BreakHitResult` (`PlayerController.GetHitResultUnderCursorByChannel` (`GameplayStatics.GetPlayerController` 0) "TraceTypeQuery1" true)))
  (bind (_outhit _returnvalue) (`KismetSystemLibrary.LineTraceSingle` (stale `self.ReceiveBeginPlay` _output_get) _location "TraceTypeQuery1" :!label _label))
  (if _returnvalue
    (bind (_bblockinghit_2 _binitialoverlap_2 _time_2 _location_2 _impactpoint _normal _impactnormal _physmat _hitactor) (`GameplayStatics.BreakHitResult` _outhit))
    (`GameplayStatics.ApplyDamage` _hitactor (`self.Weapon Damage`))
    (set `self.BeamTarget` _location_2)
    (else
      (set `self.BeamTarget` _location)))
  (`ParticleSystemComponent.SetBeamSourcePoint` (`self.ReaperBeam`) 0 (stale `self.ReceiveBeginPlay` _output_get) 0)
  (`ParticleSystemComponent.SetBeamTargetPoint` (`self.ReaperBeam`) 0 (`self.BeamTarget`) 0)
  (`KismetSystemLibrary.Delay` 0.05)
  (`self.K2_DestroyActor`))

(event `self.ReceiveBeginPlay`
  (bind _asbp_player_ship (cast `/Game/StarTempest/Characters/PlayerShip/BP_PlayerShip` (`GameplayStatics.GetPlayerCharacter` 0)))
  (bind _output_get (set `self.ShipLocation` (`SceneComponent.K2_GetComponentLocation` (`/Game/StarTempest/Characters/PlayerShip/BP_PlayerShip.PlayerShipMesh` _asbp_player_ship))))
  (goto _label))

(fn `UserConstructionScript`)
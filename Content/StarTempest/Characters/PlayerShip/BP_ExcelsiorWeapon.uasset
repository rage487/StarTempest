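; BP_ExcelsiorWeapon is a player ship weapon actor, apparently a twin shot, made of two cylinders that damage what they overlap.
; Each cylinder's overlap applies WeaponDamage to the other actor, credited to player controller 0 as both instigator and causer, then destroys that cylinder.
; The actor destroys itself once both cylinders are gone, so each can hit independently.
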(event `self.Cylinder.OnComponentBeginOverlap`
  (params (OverlappedComponent :type "PrimitiveComponent Object Reference") (OtherActor :type "Actor Object Reference") (OtherComp :type "PrimitiveComponent Object Reference") (OtherBodyIndex :type Integer) (bFromSweep :type Boolean) (SweepResult :type "HitResult Structure (by ref)"))
  (bind _returnvalue (`GameplayStatics.GetPlayerController` 0))
  (`GameplayStatics.ApplyDamage` OtherActor (`self.WeaponDamage`) _returnvalue _returnvalue)
  (`ActorComponent.K2_DestroyComponent` (`self.Cylinder`))
  (if (not (`KismetSystemLibrary.IsValid` (`self.Cylinder2`)))
    (`self.K2_DestroyActor`)))

(event `self.Cylinder2.OnComponentBeginOverlap`
  (params (OverlappedComponent :type "PrimitiveComponent Object Reference") (OtherActor :type "Actor Object Reference") (OtherComp :type "PrimitiveComponent Object Reference") (OtherBodyIndex :type Integer) (bFromSweep :type Boolean) (SweepResult :type "HitResult Structure (by ref)"))
  (bind _returnvalue (`GameplayStatics.GetPlayerController` 0))
  (`GameplayStatics.ApplyDamage` OtherActor (`self.WeaponDamage`) _returnvalue _returnvalue)
  (`ActorComponent.K2_DestroyComponent` (`self.Cylinder2`))
  (if (not (`KismetSystemLibrary.IsValid` (`self.Cylinder`)))
    (`self.K2_DestroyActor`)))

(fn `UserConstructionScript`)
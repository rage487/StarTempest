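; BP_Fodder is a Star Tempest fodder enemy that can be shot down or destroyed by ramming the player's ship.
; Incoming damage reduces AIHealth, and at zero it passes its death particle, sound, type and transform to GM_TopDown's EnemyDestroyedEvent.
; On cube overlap, it casts the other actor to the player controller's current ship class, deals fixed damage to it, then zeroes its own health and triggers the same death call.
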(event `self.ReceiveAnyDamage`
  (params (Damage :type "Float (single-precision)") (DamageType :type "DamageType Object Reference") (InstigatedBy :type "Controller Object Reference") (DamageCauser :type "Actor Object Reference"))
  ;[1 1 1] Fodder Taking Damage
  (set `self.AIHealth` (- (`self.AIHealth`) Damage))
  (if (<= (`self.AIHealth`) 0.0)
    (`self.CallDeathFunction`)))

(event `self.Cube.OnComponentBeginOverlap`
  (params (OverlappedComponent :type "PrimitiveComponent Object Reference") (OtherActor :type "Actor Object Reference") (OtherComp :type "PrimitiveComponent Object Reference") (OtherBodyIndex :type Integer) (bFromSweep :type Boolean) (SweepResult :type "HitResult Structure (by ref)"))
  ;[1 1 1] Fodder Collision with Player
  (bind _aspc_top_down (cast `/Game/StarTempest/Core/PC_TopDown` (`GameplayStatics.GetPlayerController` 0)))
  (switch `/Game/StarTempest/Characters/E_PlayerShips` (`/Game/StarTempest/Core/PC_TopDown.CurrentShip` _aspc_top_down)
    (:`NewEnumerator0`
      (cast `/Game/StarTempest/Characters/PlayerShips/Corsair/BP_Corsair` OtherActor))
    (:`NewEnumerator1`
      (cast `/Game/StarTempest/Characters/PlayerShips/Crusader/BP_Crusader` OtherActor))
    (:`NewEnumerator2`
      (cast `/Game/StarTempest/Characters/PlayerShips/Dragonfly/BP_Dragonfly` OtherActor))
    (:`NewEnumerator3`
      (cast `/Game/StarTempest/Characters/PlayerShips/Hunter/BP_Hunter` OtherActor))
    (:`NewEnumerator4`
      (cast `/Game/StarTempest/Characters/PlayerShips/Juggernaut/BP_Juggernaut` OtherActor))
    (:`NewEnumerator5`
      (cast `/Game/StarTempest/Characters/PlayerShips/Nebula/BP_Nebula` OtherActor))
    (:`NewEnumerator6`
      (cast `/Game/StarTempest/Characters/PlayerShips/Reaper/BP_Reaper` OtherActor))
    (:`NewEnumerator7`
      (cast `/Game/StarTempest/Characters/PlayerShips/Spectre/BP_Spectre` OtherActor))
    (:`NewEnumerator8`
      (cast `/Game/StarTempest/Characters/PlayerShips/Voidwalker/BP_Voidwalker` OtherActor)))
  (`GameplayStatics.ApplyDamage` OtherActor 50.0 (`GameplayStatics.GetPlayerController` 0) self)
  (set `self.AIHealth` 0.0)
  (if (<= (`self.AIHealth`) 0.0)
    (`self.CallDeathFunction`)))

(fn `CallDeathFunction`
  (bind _asgm_top_down (cast `/Game/StarTempest/Core/GM_TopDown` (`GameplayStatics.GetGameMode`)))
  (`/Game/StarTempest/Core/GM_TopDown.EnemyDestroyedEvent` _asgm_top_down (`self.DeathParticle`) (`self.DeathSound`) (`self.EnemyType`) (`self.GetTransform`) self))

(fn `UserConstructionScript`)